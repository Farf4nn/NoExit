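; BP_NPC is a lab NPC that detects the first-person player by sight and noises by hearing through PawnSensing.
; Sense events set seen or heard flags, and retriggerable 0.2-second delays clear them once stimuli stop.
; Hearing stores the noise location, while the sight handler leaves SeeEnemy empty.
; Tick only prints the current state as Spanish debug text, prioritizing sight over hearing.
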(event `self.PawnSensing.OnSeePawn`
  (params (Pawn :type "Pawn Object Reference"))
  (`self.GetEnemy` Pawn)
  (`KismetSystemLibrary.RetriggerableDelay` 0.2)
  (`self.ResetEnemy` null))

(event `self.PawnSensing.OnHearNoise`
  (params (Instigator :type "Pawn Object Reference") (Location :type "Vector Structure (by ref)") (Volume :type "Float (single-precision)"))
  (`self.GetEnemyListen` Location)
  (`KismetSystemLibrary.RetriggerableDelay` 0.2)
  (`self.RestListen`))

(event `self.ReceiveTick`
  (params (DeltaSeconds :type "Float (single-precision)"))
  (if (`self.ISeeEnemy`)
    (`KismetSystemLibrary.PrintString` "Te veo, aña" true true (struct :`G` 0.66 :`B` 1.0 :`A` 1.0) 50000000.0)
    (elif (`self.IListenEnemy`)
      (`KismetSystemLibrary.PrintString` "Te Escucho" true true (struct :`G` 0.66 :`B` 1.0 :`A` 1.0) 50000000.0)
      (else
        (`KismetSystemLibrary.PrintString` "No te veo,  OnO" true true (struct :`G` 0.66 :`B` 1.0 :`A` 1.0) 50000000.0)))))

(fn `GetEnemy`
  (params (Enemy :type "Actor Object Reference"))
  (cast `/Game/FirstPerson/Blueprints/BP_FirstPersonCharacter` Enemy)
  (set `self.SeeEnemy` null)
  (set `self.ISeeEnemy` true))

(fn `GetEnemyListen`
  (params (`Position Listen` :type "Vector Structure"))
  (set `self.PositionListen` `Position Listen`)
  (set `self.IListenEnemy` true))

(fn `ResetEnemy`
  (params (Null :type "/Game/FirstPerson/Blueprints/BP_FirstPersonCharacter Object Reference"))
  (set `self.SeeEnemy` Null)
  (set `self.ISeeEnemy` false))

(fn `RestListen`
  (set `self.IListenEnemy` false)
  (set `self.PositionListen` (0.0 0.0 0.0)))

(fn `UserConstructionScript`)